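; EnemyCube is an enemy that chases the player on sight.
; Its PawnSensing See Pawn event casts the seen pawn to FirstPersonCharacter and, on success, uses AI MoveTo to move toward it.
; A disconnected chain that lowers EnemyHealth, prints it and destroys the actor at zero or below never runs, so the cube takes no damage in this graph.
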(event `self.PawnSensing.OnSeePawn`
  (params (Pawn :type "Pawn Object Reference"))
  (bind _asfirst_person_character (cast `/Game/FirstPersonBP/Blueprints/FirstPersonCharacter` Pawn))
  (`|AIMoveTo` self (0.0 0.0 0.0) _asfirst_person_character))

(fn `UserConstructionScript`)